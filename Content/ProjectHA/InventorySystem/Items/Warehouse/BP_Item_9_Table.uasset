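; Warehouse table item that slides aside once when interacted with, playing a moving sound.
; A timeline lerps the mesh to a fixed offset, flags it as moved and repoints ItemInfo to another ItemTable row.
; Interact also writes the item's row-indexed entry in the GameState's ItemExists array.
; Check and Interact respect the moved flag, and LoadItem restores the moved state instantly without animation.
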(event Custom|Move
  (bind _새_트랙_0 (Timeline|타임라인 Play)
    (:Update
      (Transformation|SetRelativeLocation (Variables|Default|GetStaticMesh) (Math|Vector|Lerp(Vector) "0, 0, 0" "-150.000000,70.000000,0.000000" _새_트랙_0) false false)
      (Variables|Default|SetIsMoving true)
      (Variables|Default|SetItemInfo (Utilities|Struct|MakeDataTableRowHandle "/Game/ProjectHA/InventorySystem/ItemTable.ItemTable" "5")))))

(fn ConstructionScript
  (|CallParentFunction))

(fn Interact
  (params (Interactor :type Character%20Object%20Reference))
  (if (not (Variables|Default|GetIsMoving))
    (CallFunction|Move)
    (Audio|PlaySound2D "/Game/ProjectHA/InventorySystem/Items/EffectSound/chair-moving-58993__cut_1sec_.chair-moving-58993__cut_1sec_" 1.0 1.0 0.0 0 0)
    (bind _asbp_gs_main (Utilities|Casting|CastToBP_GS_Main (Game|GetGameState)))
    (Utilities|Array|SetArrayElem (Variables|/Game/ProjectHA/Game/BP_GS_Main.BP_GS_Main_C|GetItemExists _asbp_gs_main) (Math|Conversions|ToInteger(Byte) (Utilities|String|ToString(Name) (.RowName (Utilities|Struct|BreakDataTableRowHandle (Variables|Default|GetItemInfo))))) false)
    (return true)))

(fn Check
  (|CallParentFunction)
  (if (Variables|Default|GetIsMoving)
    (return false)
    (else
      (return true))))

(fn LoadItem
  (Transformation|SetRelativeLocation (Variables|Default|GetStaticMesh) "-150.000000,70.000000,0.000000" false false)
  (Variables|Default|SetIsMoving true)
  (Variables|Default|SetItemInfo (Utilities|Struct|MakeDataTableRowHandle "/Game/ProjectHA/InventorySystem/ItemTable.ItemTable" "5")))