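; Warehouse vent puzzle item that the player opens with a specific inventory item, then uses as a passage.
; Check allows interaction once opened or while that item is selected; the first Interact plays a screwdriver sound, swaps material and item row.
; The next Interact records the puzzle and item state in BP_GS_Main, switches rows again and teleports the player to a hardcoded location.
; LoadItem reapplies the final row and swapped material.
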(event EventBeginPlay
  (|CallParentFunction) ; 지금 이 노드는 비활성 상태입니다. \n핀을 끌어서 다른 노드를 연결하면 활성화됩니다.
)

(event Collision|EventActorBeginOverlap
  (params (OtherActor :type Actor%20Object%20Reference))
  (|CallParentFunction OtherActor) ; 지금 이 노드는 비활성 상태입니다. \n핀을 끌어서 다른 노드를 연결하면 활성화됩니다.
)

(event EventTick
  (params (DeltaSeconds :type Float%20%28single-precision%29))
  (|CallParentFunction DeltaSeconds) ; 지금 이 노드는 비활성 상태입니다. \n핀을 끌어서 다른 노드를 연결하면 활성화됩니다.
)

(fn ConstructionScript
  (|CallParentFunction))

(fn Interact
  (params (Interactor :type Character%20Object%20Reference))
  (if (Variables|Default|GetCondition)
    (bind _asbp_gs_main (Utilities|Casting|CastToBP_GS_Main (Game|GetGameState)))
    (Utilities|Array|SetArrayElem (Variables|/Game/ProjectHA/Game/BP_GS_Main.BP_GS_Main_C|GetPuzzleCleared _asbp_gs_main) 1 true)
    (Utilities|Array|SetArrayElem (Variables|/Game/ProjectHA/Game/BP_GS_Main.BP_GS_Main_C|GetItemExists _asbp_gs_main) (- (Math|Conversions|ToInteger(Byte) (Utilities|String|ToString(Name) (.RowName (Utilities|Struct|BreakDataTableRowHandle (Variables|Default|GetItemInfo))))) 1) false)
    (Variables|Default|SetItemInfo (Utilities|Struct|MakeDataTableRowHandle "/Game/ProjectHA/InventorySystem/ItemTable.ItemTable" "76"))
    (bind _asbp_player (Utilities|Casting|CastToBP_Player (Game|GetPlayerCharacter 0)))
    (Transformation|Teleport _asbp_player "-12310.000000,-10385.000000,4500.000000" "0, 0, 0")
    (else
      (Audio|PlaySound2D "/Game/ProjectHA/InventorySystem/Items/EffectSound/skrow-driver-38024.skrow-driver-38024" 2.0 1.0 0.0 0 0)
      (Variables|Default|SetItemInfo (Utilities|Struct|MakeDataTableRowHandle "/Game/ProjectHA/InventorySystem/ItemTable.ItemTable" "11"))
      (Rendering|Material|SetMaterial (Variables|Default|GetStaticMesh) 0 "/Game/Developing_AssetTest/Pot/Dako_glass_cooker.Dako_glass_cooker")
      (Variables|Default|SetCondition true)
      (return true))))

(fn Check
  (|CallParentFunction)
  (if (Variables|Default|GetCondition)
    (return true)
    (else
      (bind _asbp_player (Utilities|Casting|CastToBP_Player (Game|Player|GetPlayerPawn 0)))
      (if (== (.ID (Utilities|Struct|BreakItemStruct (Variables|/Game/ProjectHA/InventorySystem/BP_Inventory_Component.BP_Inventory_Component_C|GetSelectedItem (Variables|/Game/ProjectHA/Game/Character/BP_Player.BP_Player_C|GetInventory%20Component _asbp_player)))) 8)
        (return true)
        (else
          (return false))))))

(fn LoadItem
  (Variables|Default|SetItemInfo (Utilities|Struct|MakeDataTableRowHandle "/Game/ProjectHA/InventorySystem/ItemTable.ItemTable" "76"))
  (Rendering|Material|SetMaterial (Variables|Default|GetStaticMesh) 0 "/Game/Developing_AssetTest/Pot/Dako_glass_cooker.Dako_glass_cooker"))