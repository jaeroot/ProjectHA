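; Warehouse work log item that the player interacts with to inspect it in a focused view.
; Interact has the player possess the default pawn, registers the item as that character's FocusItem and blends the camera to the item.
; It then sets its Box to overlap the Visibility channel and enables the mouse cursor with Game and UI input.
; PlaySound and LoadItem are empty stubs, and the event graph is inactive.
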(event EventBeginPlay
  (|CallParentFunction) ; 지금 이 노드는 비활성 상태입니다. \n핀을 끌어서 다른 노드를 연결하면 활성화됩니다.
)

(event Collision|EventActorBeginOverlap
  (params (OtherActor :type Actor%20Object%20Reference))
  (|CallParentFunction OtherActor) ; 지금 이 노드는 비활성 상태입니다. \n핀을 끌어서 다른 노드를 연결하면 활성화됩니다.
)

(event EventTick
  (params (DeltaSeconds :type Float%20%28single-precision%29))
  (|CallParentFunction DeltaSeconds) ; 지금 이 노드는 비활성 상태입니다. \n핀을 끌어서 다른 노드를 연결하면 활성화됩니다.
)

(fn ConstructionScript
  (|CallParentFunction))

(fn PlaySound
  (params (Interactor :type Character%20Object%20Reference))
  (return false))

(fn Interact
  (params (Interactor :type Character%20Object%20Reference))
  (bind _returnvalue (Game|GetPlayerController 0))
  (bind _self self)
  (bind _asbp_player (Utilities|Casting|CastToBP_Player Interactor))
  (Default|PossessDefaultPawn _asbp_player)
  (bind _asbp_default_character (Utilities|Casting|CastToBP_DefaultCharacter (Game|Player|GetPlayerPawn 0)))
  (Variables|/Game/ProjectHA/Game/Character/BP_DefaultCharacter.BP_DefaultCharacter_C|SetFocusItem _asbp_default_character _self)
  (Game|Player|SetViewTargetwithBlend _returnvalue _self 0.5 "VTBlend_EaseIn" 0.0 false)
  (Collision|SetCollisionResponsetoChannel (Variables|Default|GetBox) "ECC_Visibility" "ECR_Overlap")
  (Variables|/Script/Engine.PlayerController|SetbShowMouseCursor _returnvalue true)
  (Input|SetInputModeGameandUI _returnvalue 0 "DoNotLock" true false)
  (return true))

(fn LoadItem)