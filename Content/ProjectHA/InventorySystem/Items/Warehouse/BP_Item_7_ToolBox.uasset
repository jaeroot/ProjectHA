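; BP_Item_7_ToolBox is the toolbox pickup item in the inventory system's Warehouse set.
; On Interact it plays a 2D pickup sound, destroys itself and updates its entry in the ItemExists array on BP_GS_Main, the game state.
; The array index comes from converting the ItemInfo row name to an integer, so the row name must be numeric.
; The event graph holds only disabled default events.
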(event EventBeginPlay
  (|CallParentFunction) ; 지금 이 노드는 비활성 상태입니다. \n핀을 끌어서 다른 노드를 연결하면 활성화됩니다.
)

(event Collision|EventActorBeginOverlap
  (params (OtherActor :type Actor%20Object%20Reference))
  (|CallParentFunction OtherActor) ; 지금 이 노드는 비활성 상태입니다. \n핀을 끌어서 다른 노드를 연결하면 활성화됩니다.
)

(event EventTick
  (params (DeltaSeconds :type Float%20%28single-precision%29))
  (|CallParentFunction DeltaSeconds) ; 지금 이 노드는 비활성 상태입니다. \n핀을 끌어서 다른 노드를 연결하면 활성화됩니다.
)

(fn ConstructionScript
  (|CallParentFunction))

(fn Interact
  (params (Interactor :type Character%20Object%20Reference))
  (Audio|PlaySound2D "/Game/ProjectHA/InventorySystem/Items/EffectSound/gift_pickup.gift_pickup" 1.0 1.0 0.0 0 0)
  (Actor|DestroyActor)
  (bind _asbp_gs_main (Utilities|Casting|CastToBP_GS_Main (Game|GetGameState)))
  (Utilities|Array|SetArrayElem (Variables|/Game/ProjectHA/Game/BP_GS_Main.BP_GS_Main_C|GetItemExists _asbp_gs_main) (Math|Conversions|ToInteger(Byte) (Utilities|String|ToString(Name) (.RowName (Utilities|Struct|BreakDataTableRowHandle (Variables|Default|GetItemInfo))))) false)
  (return true))