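; BP_Item_62_Woodbox is an interactable wooden box item that the player breaks.
; Check calls the parent, then passes if Condition is set or the player's selected inventory item has ID 63.
; Interact triggers the Destory event, which plays a crash sound and waits two seconds before destroying the actor.
; Before destruction, it clears its ItemExists entry in BP_GS_Main, indexed by its row name.
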(event Custom|Destory
  (Audio|PlaySound2D "/Game/ProjectHA/InventorySystem/Items/EffectSound/SQ_WoodCrash.SQ_WoodCrash" 1.0 1.0 0.0 0 0)
  (Utilities|FlowControl|Delay 2.0)
  (bind _asbp_gs_main (Utilities|Casting|CastToBP_GS_Main (Game|GetGameState)))
  (Utilities|Array|SetArrayElem (Variables|/Game/ProjectHA/Game/BP_GS_Main.BP_GS_Main_C|GetItemExists _asbp_gs_main) (Math|Conversions|ToInteger(Byte) (Utilities|String|ToString(Name) (.RowName (Utilities|Struct|BreakDataTableRowHandle (Variables|Default|GetItemInfo))))) false)
  (Actor|DestroyActor))

(event EventBeginPlay
  (|CallParentFunction) ; 지금 이 노드는 비활성 상태입니다. \n핀을 끌어서 다른 노드를 연결하면 활성화됩니다.
)

(event Collision|EventActorBeginOverlap
  (params (OtherActor :type Actor%20Object%20Reference))
  (|CallParentFunction OtherActor) ; 지금 이 노드는 비활성 상태입니다. \n핀을 끌어서 다른 노드를 연결하면 활성화됩니다.
)

(event EventTick
  (params (DeltaSeconds :type Float%20%28single-precision%29))
  (|CallParentFunction DeltaSeconds) ; 지금 이 노드는 비활성 상태입니다. \n핀을 끌어서 다른 노드를 연결하면 활성화됩니다.
)

(fn ConstructionScript
  (|CallParentFunction))

(fn Interact
  (params (Interactor :type Character%20Object%20Reference))
  (CallFunction|Destory)
  (return true))

(fn Check
  (|CallParentFunction)
  (if (Variables|Default|GetCondition)
    (return true)
    (else
      (bind _asbp_player (Utilities|Casting|CastToBP_Player (Game|Player|GetPlayerPawn 0)))
      (if (== (.ID (Utilities|Struct|BreakItemStruct (Variables|/Game/ProjectHA/InventorySystem/BP_Inventory_Component.BP_Inventory_Component_C|GetSelectedItem (Variables|/Game/ProjectHA/Game/Character/BP_Player.BP_Player_C|GetInventory%20Component _asbp_player)))) 63)
        (return true)
        (else
          (return false))))))