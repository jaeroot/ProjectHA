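; BP_Message_08 is a forest message item in the inventory system that records message number 8 in the game state.
; Its Check override casts the game state to BP_GS_Main, sets that index of the Message array to true, and returns false.
; The event graph holds only disabled default events, and the construction script just calls the parent.
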(event EventBeginPlay
  (|CallParentFunction) ; 지금 이 노드는 비활성 상태입니다. \n핀을 끌어서 다른 노드를 연결하면 활성화됩니다.
)

(event Collision|EventActorBeginOverlap
  (params (OtherActor :type Actor%20Object%20Reference))
  (|CallParentFunction OtherActor) ; 지금 이 노드는 비활성 상태입니다. \n핀을 끌어서 다른 노드를 연결하면 활성화됩니다.
)

(event EventTick
  (params (DeltaSeconds :type Float%20%28single-precision%29))
  (|CallParentFunction DeltaSeconds) ; 지금 이 노드는 비활성 상태입니다. \n핀을 끌어서 다른 노드를 연결하면 활성화됩니다.
)

(fn ConstructionScript
  (|CallParentFunction))

(fn Check
  (bind _asbp_gs_main (Utilities|Casting|CastToBP_GS_Main (Game|GetGameState)))
  (Utilities|Array|SetArrayElem (Variables|/Game/ProjectHA/Game/BP_GS_Main.BP_GS_Main_C|GetMessage _asbp_gs_main) 8 true)
  (return false))