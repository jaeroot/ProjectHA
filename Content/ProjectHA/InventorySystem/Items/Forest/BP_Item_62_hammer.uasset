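; BP_Item_62_hammer is the hammer item Blueprint in the Forest set of the inventory system, with no active logic of its own.
; Its Destory event is empty, the other events are disabled parent-call stubs, and its construction script only calls the parent.
; Disconnected leftover nodes would play a wood-crash sound before a delayed destroy, or update the game state's ItemExists array by row-name index.
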(event Custom|Destory)

(event EventBeginPlay
  (|CallParentFunction) ; 지금 이 노드는 비활성 상태입니다. \n핀을 끌어서 다른 노드를 연결하면 활성화됩니다.
)

(event Collision|EventActorBeginOverlap
  (params (OtherActor :type Actor%20Object%20Reference))
  (|CallParentFunction OtherActor) ; 지금 이 노드는 비활성 상태입니다. \n핀을 끌어서 다른 노드를 연결하면 활성화됩니다.
)

(event EventTick
  (params (DeltaSeconds :type Float%20%28single-precision%29))
  (|CallParentFunction DeltaSeconds) ; 지금 이 노드는 비활성 상태입니다. \n핀을 끌어서 다른 노드를 연결하면 활성화됩니다.
)

(fn ConstructionScript
  (|CallParentFunction))