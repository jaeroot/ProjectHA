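; BP_Inventory_Component is an inventory component that stores picked-up item structs and drives the player's inventory UI.
; AddToInventory appends an item to the Inventory array, then has the inventory widget on BP_PC_Main's main widget create its boxes from this component.
; ToggleInventory flips that widget's inventory visibility and uses the result to set the mouse cursor and switch between Game-and-UI and Game-Only input modes.
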(event EventBeginPlay)

(event EventTick
  (params (DeltaSeconds :type Float%20%28single-precision%29)))

(fn ToggleInventory
  (bind _returnvalue (Game|GetPlayerController 0))
  (bind _asbp_pc_main (Utilities|Casting|CastToBP_PC_Main _returnvalue))
  (Utilities|IsValid (Variables|/Game/ProjectHA/Game/BP_PC_Main.BP_PC_Main_C|GetWB_Main_Ref _asbp_pc_main)
    (:Is%20Valid
      (bind _showmouse (Default|SetVisibilityInventory (Variables|/Game/ProjectHA/Game/BP_PC_Main.BP_PC_Main_C|GetWB_Main_Ref _asbp_pc_main)))
      (bind _output_get (Variables|/Script/Engine.PlayerController|SetbShowMouseCursor _returnvalue _showmouse))
      (if _output_get
        (Input|SetInputModeGameandUI _returnvalue (Variables|/Game/ProjectHA/Game/BP_PC_Main.BP_PC_Main_C|GetWB_Main_Ref _asbp_pc_main) "DoNotLock" true false)
        (else
          (Input|SetInputModeGameOnly _returnvalue false))))))

(fn AddtoInventory
  (params (Item :type Item%20Struct%20Structure))
  (bind (_id _name _canactivate _script _thumbnail _class) (Utilities|Struct|BreakItemStruct Item))
  (Utilities|Array|Add (Variables|Default|GetInventory) (Utilities|Struct|MakeItemStruct _id _name _canactivate _script _thumbnail _class))
  (bind _asbp_pc_main (Utilities|Casting|CastToBP_PC_Main (Game|GetPlayerController 0)))
  (Utilities|IsValid (Variables|/Game/ProjectHA/Game/BP_PC_Main.BP_PC_Main_C|GetWB_Main_Ref _asbp_pc_main)
    (:Is%20Valid
      (Default|CreateInventoryBox (Variables|/Game/ProjectHA/UI/WB_Main.WB_Main_C|GetWB_Inventory (Variables|/Game/ProjectHA/Game/BP_PC_Main.BP_PC_Main_C|GetWB_Main_Ref _asbp_pc_main)) self))))