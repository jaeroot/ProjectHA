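; BP_GS_Main is the main game state, holding flag arrays for item existence, puzzle clears, story and messages.
; Its construction script copies the arrays from the BP_HA_GI save instance when LoadData is set.
; Otherwise it rebuilds them by probing each data table for numbered row names until one is missing.
; Rebuilt items default to true and the other flags to false, except one puzzle entry preset as cleared.
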(event EventBeginPlay)

(event EventTick
  (params (DeltaSeconds :type Float%20%28single-precision%29)))

(fn ConstructionScript
  (bind _asbp_ha_gi (Utilities|Casting|CastToBP_HA_GI (Game|GetGameInstance)))
  (if (Variables|/Game/ProjectHA/Game/BP_HA_GI.BP_HA_GI_C|GetLoadData? _asbp_ha_gi)
    (Variables|Item|SetItemExists (Variables|/Game/ProjectHA/Game/BP_HA_SG.BP_HA_SG_C|GetItemExists (Variables|/Game/ProjectHA/Game/BP_HA_GI.BP_HA_GI_C|GetSave%20Game%20Instance _asbp_ha_gi)))
    (Variables|Puzzle|SetPuzzleCleared (Variables|/Game/ProjectHA/Game/BP_HA_SG.BP_HA_SG_C|GetPuzzleCleared (Variables|/Game/ProjectHA/Game/BP_HA_GI.BP_HA_GI_C|GetSave%20Game%20Instance _asbp_ha_gi)))
    (Variables|Puzzle|SetStory (Variables|/Game/ProjectHA/Game/BP_HA_SG.BP_HA_SG_C|GetStory (Variables|/Game/ProjectHA/Game/BP_HA_GI.BP_HA_GI_C|GetSave%20Game%20Instance _asbp_ha_gi)))
    (Variables|Puzzle|SetMessage (Variables|/Game/ProjectHA/Game/BP_HA_SG.BP_HA_SG_C|GetMessage (Variables|/Game/ProjectHA/Game/BP_HA_GI.BP_HA_GI_C|GetSave%20Game%20Instance _asbp_ha_gi)))
    (else
      (Utilities|FlowControl|Sequence
        (:then_0
          (Variables|Item|SetItemCount 0)
          (Utilities|Array|Clear (Variables|Item|GetItemExists))
          (CallFunction|SearchItemExists)
          (while (Variables|Item|GetItemCountFlag)
            (CallFunction|SearchItemExists)))
        (:then_1
          (Variables|Puzzle|SetPuzzleCount 0)
          (Utilities|Array|Clear (Variables|Puzzle|GetPuzzleCleared))
          (CallFunction|SearchPuzzleExists)
          (while (Variables|Puzzle|GetPuzzleCountFlag)
            (CallFunction|SearchPuzzleExists))
          (Utilities|Array|SetArrayElem (Variables|Puzzle|GetPuzzleCleared) 0 true))
        (:then_2
          (Variables|Puzzle|SetStoryCount 0)
          (Utilities|Array|Clear (Variables|Puzzle|GetStory))
          (CallFunction|SearchStoryExists)
          (while (Variables|Puzzle|GetStoryCountFlag)
            (CallFunction|SearchStoryExists))
          (Utilities|Array|SetArrayElem (Variables|Puzzle|GetStory) 0 false))
        (:then_3
          (Variables|Puzzle|SetMessageCount 0)
          (Utilities|Array|Clear (Variables|Puzzle|GetMessage))
          (CallFunction|SearchMessageExists)
          (while (Variables|Puzzle|GetMessageCountFlag)
            (CallFunction|SearchMessageExists))
          (Utilities|Array|SetArrayElem (Variables|Puzzle|GetMessage) 0 false))))))

(fn SearchItemExists
  (bind _result (Math|Integer|IncrementInt (Variables|Item|GetItemCount))
    (:%20%20
      (bind _returnvalue (Class|DataTableFunctionLibrary|DoesDataTableRowExist "/Game/ProjectHA/InventorySystem/ItemTable.ItemTable" (Utilities|String|StringToName (Utilities|String|ToString(Integer) _result))))
      (bind _output_get (Variables|Item|SetItemCountFlag _returnvalue))
      (Utilities|Array|Add (Variables|Item|GetItemExists) true)
      (if (not _output_get)
        (Math|Integer|DecrementInt (Variables|Item|GetItemCount))))))

(fn SearchPuzzleExists
  (bind _result (Math|Integer|IncrementInt (Variables|Puzzle|GetPuzzleCount))
    (:%20%20
      (bind _returnvalue (Class|DataTableFunctionLibrary|DoesDataTableRowExist "/Game/ProjectHA/Puzzle/PuzzleTable.PuzzleTable" (Utilities|String|StringToName (Utilities|String|ToString(Integer) _result))))
      (bind _output_get (Variables|Puzzle|SetPuzzleCountFlag _returnvalue))
      (Utilities|Array|Add (Variables|Puzzle|GetPuzzleCleared) false)
      (if (not _output_get)
        (Math|Integer|DecrementInt (Variables|Puzzle|GetPuzzleCount))))))

(fn SearchStoryExists
  (bind _result (Math|Integer|IncrementInt (Variables|Puzzle|GetStoryCount))
    (:%20%20
      (bind _returnvalue (Class|DataTableFunctionLibrary|DoesDataTableRowExist "/Game/ProjectHA/Story/StoryTable.StoryTable" (Utilities|String|StringToName (Utilities|String|ToString(Integer) _result))))
      (bind _output_get (Variables|Puzzle|SetStoryCountFlag _returnvalue))
      (Utilities|Array|Add (Variables|Puzzle|GetStory) false)
      (if (not _output_get)
        (Math|Integer|DecrementInt (Variables|Puzzle|GetStoryCount))))))

(fn SearchMessageExists
  (bind _result (Math|Integer|IncrementInt (Variables|Puzzle|GetMessageCount))
    (:%20%20
      (bind _returnvalue (Class|DataTableFunctionLibrary|DoesDataTableRowExist "/Game/ProjectHA/Story/MessageTable.MessageTable" (Utilities|String|StringToName (Utilities|String|ToString(Integer) _result))))
      (bind _output_get (Variables|Puzzle|SetMessageCountFlag _returnvalue))
      (Utilities|Array|Add (Variables|Puzzle|GetMessage) false)
      (if (not _output_get)
        (Math|Integer|DecrementInt (Variables|Puzzle|GetMessageCount))))))