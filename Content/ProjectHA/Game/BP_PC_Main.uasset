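; Main player controller that owns and displays the game's UI widgets: main, pause, story, option and hint screens.
; BeginPlay creates the main widget and adds it to the viewport.
; Separate functions lazily create and cache each of the other widgets, add them to the viewport and switch input to UI-only focused on that widget.
; The pause function also shows the mouse cursor and pauses the game.
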(event EventBeginPlay
  (bind _returnvalue (UserInterface|CreateWidget "/Game/ProjectHA/UI/WB_Main.WB_Main_C" (Game|GetPlayerController 0)))
  (bind _output_get (Variables|Default|SetWB_Main_Ref _returnvalue))
  (UserInterface|Viewport|AddtoViewport _output_get 0))

(fn ConstructionScript)

(fn CreatePauseWidget
  (bind _self self)
  (bind _wb_pause_ref (Variables|BP_PC_Main_C|GetWB_Pause_Ref _self)
    (:then
      _)
    (:else
      (bind _returnvalue (UserInterface|CreateWidget "/Game/ProjectHA/UI/WB_Pause.WB_Pause_C" _self))
      (Variables|Default|SetWB_Pause_Ref _returnvalue)))
  (Variables|/Script/Engine.PlayerController|SetbShowMouseCursor _self true)
  (UserInterface|Viewport|AddtoViewport _wb_pause_ref 0)
  (Input|SetInputModeUIOnly _self _wb_pause_ref "DoNotLock" false)
  (Game|SetGamePaused true))

(fn CreateStoryWidget
  (bind _self self)
  (bind _wb_story_ref (Variables|Default|GetWB_Story_Ref)
    (:then
      _)
    (:else
      (bind _returnvalue (UserInterface|CreateWidget "/Game/ProjectHA/UI/Pause/WB_Story.WB_Story_C" _self))
      (Variables|Default|SetWB_Story_Ref _returnvalue)))
  (UserInterface|Viewport|AddtoViewport _wb_story_ref 0)
  (Input|SetInputModeUIOnly _self _wb_story_ref "DoNotLock" false))

(fn CreateOptionWidget
  (bind _self self)
  (bind _wb_option_ref (Variables|Default|GetWB_Option_Ref)
    (:then
      _)
    (:else
      (bind _returnvalue (UserInterface|CreateWidget "/Game/ProjectHA/UI/Pause/WB_Option.WB_Option_C" _self))
      (Variables|Default|SetWB_Option_Ref _returnvalue)))
  (UserInterface|Viewport|AddtoViewport _wb_option_ref 0)
  (Input|SetInputModeUIOnly _self _wb_option_ref "DoNotLock" false))

(fn CreateHintWidget
  (bind _self self)
  (bind _wb_hint_ref (Variables|Default|GetWB_Hint_Ref)
    (:then
      _)
    (:else
      (bind _returnvalue (UserInterface|CreateWidget "/Game/ProjectHA/UI/Pause/WB_Hint.WB_Hint_C" _self))
      (Variables|Default|SetWB_Hint_Ref _returnvalue)))
  (UserInterface|Viewport|AddtoViewport _wb_hint_ref 0)
  (Input|SetInputModeUIOnly _self _wb_hint_ref "DoNotLock" false))