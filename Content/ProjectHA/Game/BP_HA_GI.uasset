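; Game instance for ProjectHA that holds the current BP_HA_SG save object and handles creating, saving and loading it.
; Init creates a fresh save object, and Save fills it from game state progress, player inventory, transform and indoor flag, and controller BGM.
; Slot names combine the object's slot name and user index.
; Load only replaces the held object with the slot's data, without applying it to the world.
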(event EventInit
  (CallFunction|New))

(fn Save
  (bind _save_game_instance (Variables|SaveGame|GetSave%20Game%20Instance))
  (bind _save_game_instance_2 (Variables|SaveGame|GetSave%20Game%20Instance))
  (bind _save_game_instance_3 (Variables|SaveGame|GetSave%20Game%20Instance))
  (bind _save_game_instance_4 (Variables|SaveGame|GetSave%20Game%20Instance))
  (bind _saveslotname (Variables|/Game/ProjectHA/Game/BP_HA_SG.BP_HA_SG_C|GetSaveSlotName _save_game_instance))
  (bind _userindex (Variables|/Game/ProjectHA/Game/BP_HA_SG.BP_HA_SG_C|GetUserIndex _save_game_instance))
  (bind _returnvalue (Utilities|String|ToString(Integer) _userindex))
  (bind _returnvalue_2 (Utilities|String|Append _saveslotname _returnvalue))
  (Utilities|FlowControl|Sequence
    (:then_0
      (bind _asbp_gs_main (Utilities|Casting|CastToBP_GS_Main (Game|GetGameState)))
      (Variables|/Game/ProjectHA/Game/BP_HA_SG.BP_HA_SG_C|SetItemExists _save_game_instance_4 (Variables|/Game/ProjectHA/Game/BP_GS_Main.BP_GS_Main_C|GetItemExists _asbp_gs_main))
      (Variables|/Game/ProjectHA/Game/BP_HA_SG.BP_HA_SG_C|SetPuzzleCleared _save_game_instance_4 (Variables|/Game/ProjectHA/Game/BP_GS_Main.BP_GS_Main_C|GetPuzzleCleared _asbp_gs_main))
      (Variables|/Game/ProjectHA/Game/BP_HA_SG.BP_HA_SG_C|SetStory _save_game_instance_4 (Variables|/Game/ProjectHA/Game/BP_GS_Main.BP_GS_Main_C|GetStory _asbp_gs_main))
      (Variables|/Game/ProjectHA/Game/BP_HA_SG.BP_HA_SG_C|SetMessage _save_game_instance_4 (Variables|/Game/ProjectHA/Game/BP_GS_Main.BP_GS_Main_C|GetMessage _asbp_gs_main))
      (Variables|/Game/ProjectHA/Game/BP_HA_SG.BP_HA_SG_C|SetStoryAmy _save_game_instance_4 (Variables|/Game/ProjectHA/Game/BP_GS_Main.BP_GS_Main_C|GetStoryAmy _asbp_gs_main)))
    (:then_1
      (bind _asbp_player (Utilities|Casting|CastToBP_Player (Game|Player|GetPlayerPawn 0)))
      (Variables|/Game/ProjectHA/Game/BP_HA_SG.BP_HA_SG_C|SetInventory _save_game_instance_3 (Variables|/Game/ProjectHA/InventorySystem/BP_Inventory_Component.BP_Inventory_Component_C|GetInventory (Variables|/Game/ProjectHA/Game/Character/BP_Player.BP_Player_C|GetInventory%20Component _asbp_player)))
      (Variables|/Game/ProjectHA/Game/BP_HA_SG.BP_HA_SG_C|SetSelectedItem _save_game_instance_3 (Variables|/Game/ProjectHA/InventorySystem/BP_Inventory_Component.BP_Inventory_Component_C|GetSelectedItem (Variables|/Game/ProjectHA/Game/Character/BP_Player.BP_Player_C|GetInventory%20Component _asbp_player)))
      (Variables|/Game/ProjectHA/Game/BP_HA_SG.BP_HA_SG_C|SetLocation _save_game_instance_3 (.location (Transformation|GetActorTransform _asbp_player)))
      (Variables|/Game/ProjectHA/Game/BP_HA_SG.BP_HA_SG_C|SetRotation _save_game_instance_3 (.rotation (Transformation|GetActorTransform _asbp_player))))
    (:then_2
      (bind _asbp_pc_main (Utilities|Casting|CastToBP_PC_Main (Game|GetPlayerController 0)))
      (Variables|/Game/ProjectHA/Game/BP_HA_SG.BP_HA_SG_C|SetBGM _save_game_instance_2 (Variables|/Game/ProjectHA/Game/BP_PC_Main.BP_PC_Main_C|GetBGM _asbp_pc_main))
      (bind _asbp_player_2 (Utilities|Casting|CastToBP_Player (Game|Player|GetPlayerPawn 0)))
      (Variables|/Game/ProjectHA/Game/BP_HA_SG.BP_HA_SG_C|SetIsInDoor _save_game_instance_2 (Variables|/Game/ProjectHA/Game/Character/BP_Player.BP_Player_C|GetIsInDoor _asbp_player_2)))
    (:then_3
      (SaveGame|SaveGametoSlot _save_game_instance _returnvalue_2)
      (Development|PrintString (Utilities|String|Append _returnvalue_2 "에 저장 완료")))))

(fn Load
  (Utilities|FlowControl|Sequence
    (:then_0
      (bind _returnvalue (SaveGame|LoadGamefromSlot (Utilities|String|Append (Variables|/Game/ProjectHA/Game/BP_HA_SG.BP_HA_SG_C|GetSaveSlotName (Variables|SaveGame|GetSave%20Game%20Instance)) (Utilities|String|ToString(Integer) (Variables|/Game/ProjectHA/Game/BP_HA_SG.BP_HA_SG_C|GetUserIndex (Variables|SaveGame|GetSave%20Game%20Instance))))))
      (bind _asbp_ha_sg (Utilities|Casting|CastToBP_HA_SG _returnvalue))
      (Variables|SaveGame|SetSave%20Game%20Instance _asbp_ha_sg)
      (Development|PrintString (Utilities|String|Append (Utilities|String|Append (Variables|/Game/ProjectHA/Game/BP_HA_SG.BP_HA_SG_C|GetSaveSlotName (Variables|SaveGame|GetSave%20Game%20Instance)) (Utilities|String|ToString(Integer) (Variables|/Game/ProjectHA/Game/BP_HA_SG.BP_HA_SG_C|GetUserIndex (Variables|SaveGame|GetSave%20Game%20Instance)))) "에서 로딩 완료.")))))

(fn New
  (bind _returnvalue (SaveGame|CreateSaveGameObject "/Game/ProjectHA/Game/BP_HA_SG.BP_HA_SG_C"))
  (Variables|SaveGame|SetSave%20Game%20Instance _returnvalue))