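; BP_DefaultCharacter is a temporary mouse-driven pawn for clicking puzzles on a focused item.
; On possession it swaps BP_PC_Main's main widget for WB_DefaultPawn and shows the cursor.
; IA_Puzzle line-traces from the cursor and sends ClickPuzzleMessage to the hit actor with its component.
; PossessPlayerPawn restores the player pawn and FocusItem's Visibility blocking; unpossession restores the UI, hides the cursor and destroys this pawn.
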(event Input|EnhancedActionEvents|EnhancedInputActionIA_Puzzle
  (params (ActionValue :type Boolean) (ElapsedSeconds :type Float%20%28double-precision%29) (TriggeredSeconds :type Float%20%28double-precision%29) (InputAction :type Input%20Action%20Object%20Reference :default "/Game/ProjectHA/Input/Actions/IA_Puzzle.IA_Puzzle"))
  ;[1 1 1] Activate Puzzle
  (:Started
    (CallFunction|ActivatePuzzle)))

(event EventBeginPlay)

(event Collision|EventActorBeginOverlap
  (params (OtherActor :type Actor%20Object%20Reference)))

(event EventTick
  (params (DeltaSeconds :type Float%20%28single-precision%29)))

(event EventPossessed
  (params (NewController :type Controller%20Object%20Reference))
  (bind _asbp_pc_main (Utilities|Casting|CastToBP_PC_Main NewController))
  (Default|HideMainWidget _asbp_pc_main)
  (bind _returnvalue (UserInterface|CreateWidget "/Game/ProjectHA/UI/WB_DefaultPawn.WB_DefaultPawn_C" _asbp_pc_main))
  (bind _output_get (Variables|Default|SetDefaultWidget _returnvalue))
  (UserInterface|Viewport|AddtoViewport _output_get 0)
  (Variables|/Game/ProjectHA/Game/BP_PC_Main.BP_PC_Main_C|SetShowMouse? _asbp_pc_main true))

(event EventUnpossessed
  (params (OldController :type Controller%20Object%20Reference))
  (bind _asbp_pc_main (Utilities|Casting|CastToBP_PC_Main OldController))
  (Default|ShowMainWidget _asbp_pc_main)
  (Widget|RemovefromParent (Variables|Default|GetDefaultWidget))
  (Variables|/Game/ProjectHA/Game/BP_PC_Main.BP_PC_Main_C|SetShowMouse? _asbp_pc_main false)
  (Actor|DestroyActor))

(fn ConstructionScript)

(fn ActivatePuzzle
  (bind _returnvalue (Game|GetPlayerController 0))
  (bind (_worldlocation _worlddirection) (Game|Player|ConvertMouseLocationToWorldSpace _returnvalue))
  (bind (_outhit _returnvalue_2) (Collision|LineTraceByChannel _worldlocation (+ _worldlocation (* _worlddirection 5e+02)) "TraceTypeQuery1" false 0 "None"))
  (if _returnvalue_2
    (Class|BPClickPuzzle|ClickPuzzle(Message) (.HitActor (Collision|BreakHitResult _outhit)) (.HitComponent (Collision|BreakHitResult _outhit)))))

(fn PossessPlayerPawn
  (bind _playerpawn (Variables|Default|GetPlayerPawn))
  (Rendering|SetActorHiddenInGame _playerpawn false)
  (Collision|SetCollisionResponsetoChannel (Variables|/Game/ProjectHA/InventorySystem/Items/Item.Item_C|GetBox (Variables|Default|GetFocusItem)) "ECC_Visibility" "ECR_Block")
  (Pawn|Possess (Game|GetPlayerController 0) _playerpawn))